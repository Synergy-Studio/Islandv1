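; A magic circle effect actor that appears to serve as a teleport target marker.
; The Fx component takes its color from the Color variable at construction, saves it as the default, and starts deactivated on BeginPlay.
; TeleportToggle switches the effect on or off.
; TeleportColor alternates the "color" vector parameter between the default and a hardcoded green by flipping IsColorSet, and prints a debug message.
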(event EventBeginPlay
  (|CallParentFunction)
  (Components|Activation|Deactivate (Variables|Default|Getfx)))

(event Collision|EventActorBeginOverlap
  (params (OtherActor :type Actor%20Object%20Reference))
  (|CallParentFunction OtherActor) ; This node is disabled and will not be called.\nDrag off pins to build functionality.
)

(event EventTick
  (params (DeltaSeconds :type Float%20%28single-precision%29))
  (|CallParentFunction DeltaSeconds) ; This node is disabled and will not be called.\nDrag off pins to build functionality.
)

(event EventTeleportToggle
  (Components|Activation|ToggleActive (Variables|Default|Getfx)))

(event EventTeleportColor
  (Development|PrintString "Color Set!")
  (Effects|Components|ParticleSystem|SetVectorParameter (Variables|Default|Getfx) "color" (Math|Conversions|ToVector(LinearColor) (select (Variables|Default|GetIsColorSet?) (Variables|Default|GetDefaultColor) (Utilities|Struct|MakeLinearColor 0.0 255.0 0.0 0.3))))
  (if (Variables|Default|GetIsColorSet?)
    (Variables|Default|SetIsColorSet? false)
    (else
      (Variables|Default|SetIsColorSet? true))))

(fn ConstructionScript
  (bind _color (Variables|Default|Getcolor))
  (|CallParentFunction)
  (Effects|Components|ParticleSystem|SetVectorParameter (Variables|Default|Getfx) "color" (Math|Conversions|ToVector(LinearColor) _color))
  (Variables|Default|SetDefaultColor _color))