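; Magic circle actor that signals teleport availability to the MouseCharacter and to BP_ky_magicCircle_Target actors as the player enters or leaves it.
; BeginPlay caches every target actor in the level.
; Sphere begin and end overlaps, filtered to the character's capsule, both send TeleportToggleMessage to the character and all cached targets, relying on paired toggles.
; The construction script passes Color into the Fx component's color parameter.
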(event OnComponentBeginOverlap(Sphere)
  (params (OverlappedComponent :type Primitive%20Component%20Object%20Reference) (OtherActor :type Actor%20Object%20Reference) (OtherComp :type Primitive%20Component%20Object%20Reference) (OtherBodyIndex :type Integer) (bFromSweep :type Boolean) (SweepResult :type Hit%20Result%20Structure%20%28by%20ref%29))
  (bind _asmouse_character (Utilities|Casting|CastToMouseCharacter OtherActor))
  (if (== OtherComp (Variables|/Script/Engine.Character|GetCapsuleComponent _asmouse_character))
    (Class|SwitchInterface|TeleportToggle(Message) _asmouse_character)
    (for _array_element (Variables|Default|GetTargetArray)
      (Class|SwitchInterface|TeleportToggle(Message) _array_element))))

(event OnComponentEndOverlap(Sphere)
  (params (OverlappedComponent :type Primitive%20Component%20Object%20Reference) (OtherActor :type Actor%20Object%20Reference) (OtherComp :type Primitive%20Component%20Object%20Reference) (OtherBodyIndex :type Integer))
  (bind _asmouse_character (Utilities|Casting|CastToMouseCharacter OtherActor))
  (if (== OtherComp (Variables|/Script/Engine.Character|GetCapsuleComponent _asmouse_character))
    (Class|SwitchInterface|TeleportToggle(Message) _asmouse_character)
    (for _array_element (Variables|Default|GetTargetArray)
      (Class|SwitchInterface|TeleportToggle(Message) _array_element))))

(event EventBeginPlay
  (|CallParentFunction)
  (bind _outactors (Actor|GetAllActorsOfClass "/Game/Mechanics/FXVarietyPack/Blueprints/BP_ky_magicCircle_Target.BP_ky_magicCircle_Target_C"))
  (Variables|Default|SetTargetArray _outactors))

(event Collision|EventActorBeginOverlap
  (params (OtherActor :type Actor%20Object%20Reference))
  (|CallParentFunction OtherActor) ; This node is disabled and will not be called.\nDrag off pins to build functionality.
)

(event EventTick
  (params (DeltaSeconds :type Float%20%28single-precision%29))
  (|CallParentFunction DeltaSeconds) ; This node is disabled and will not be called.\nDrag off pins to build functionality.
)

(fn ConstructionScript
  (|CallParentFunction)
  (Effects|Components|ParticleSystem|SetVectorParameter (Variables|Default|Getfx) "color" (Math|Conversions|ToVector(LinearColor) (Variables|Default|Getcolor))))