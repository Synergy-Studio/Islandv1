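; Magic circle teleport point that is active by day or by night, set by its DayTP tag, with its effect following MouseCharacter's day/night switch.
; At BeginPlay it caches circles tagged for the opposite phase.
; When MouseCharacter enters during its phase, it toggles those within MaxTPDistance and sends them to the character, reversing this on exit.
; TeleportColor toggles the effect's "color" float to highlight a targeted circle.
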(event OnComponentActivated(fx)
  (params (Component :type Actor%20Component%20Object%20Reference) (bReset :type Boolean))
  (if (Math|Boolean|Equal(Boolean) (Variables|Default|GetDayOrNight) (Variables|Default|GetIsDay?))
    (Effects|Components|ParticleSystem|SetFloatParameter (Variables|Default|Getfx) "color" (Variables|Default|GetDefaultColor))))

(event OnComponentBeginOverlap(Capsule)
  (params (OverlappedComponent :type Primitive%20Component%20Object%20Reference) (OtherActor :type Actor%20Object%20Reference) (OtherComp :type Primitive%20Component%20Object%20Reference) (OtherBodyIndex :type Integer) (bFromSweep :type Boolean) (SweepResult :type Hit%20Result%20Structure%20%28by%20ref%29))
  (bind _inviewarray (Variables|Default|GetInViewArray))
  (if (Math|Boolean|Equal(Boolean) (Variables|Default|GetDayOrNight) (Variables|Default|GetIsDay?))
    (bind _asmouse_character (Utilities|Casting|CastToMouseCharacter OtherActor))
    (if (== (Variables|/Script/Engine.Character|GetCapsuleComponent _asmouse_character) OtherComp)
      (for _array_element (Variables|Default|GetTargetArray)
        (if (not (>= (Math|Vector|Distance(Vector) (Transformation|GetActorLocation (Variables|Default|GetMainChar)) (Transformation|GetActorLocation _array_element)) (Variables|Default|GetMaxTPDistance)))
          (Utilities|Array|Add _inviewarray _array_element)
          (Class|SwitchInterface|TeleportToggle(Message) _array_element)))
      (Class|SwitchInterface|2WayTeleToggle(Message) _asmouse_character _inviewarray)
      (Development|PrintString "ArraySent" true true "(R=0.000000,G=0.660000,B=1.000000,A=1.000000)" 5.0))))

(event OnComponentEndOverlap(Capsule)
  (params (OverlappedComponent :type Primitive%20Component%20Object%20Reference) (OtherActor :type Actor%20Object%20Reference) (OtherComp :type Primitive%20Component%20Object%20Reference) (OtherBodyIndex :type Integer))
  (bind _inviewarray (Variables|Default|GetInViewArray))
  (if (Math|Boolean|Equal(Boolean) (Variables|Default|GetDayOrNight) (Variables|Default|GetIsDay?))
    (bind _asmouse_character (Utilities|Casting|CastToMouseCharacter OtherActor))
    (if (== (Variables|/Script/Engine.Character|GetCapsuleComponent _asmouse_character) OtherComp)
      (for _array_element _inviewarray
        (Class|SwitchInterface|TeleportToggle(Message) _array_element))
      (Utilities|Array|Clear _inviewarray)
      (Class|SwitchInterface|2WayTeleToggle(Message) _asmouse_character _inviewarray))))

(event Custom|DayNightToggle
  (bind _fx (Variables|Default|Getfx))
  (Variables|Default|SetIsDay? (not (Variables|Default|GetIsDay?)))
  (if (Variables|Default|GetDayOrNight)
    (if (Variables|Default|GetIsDay?)
      (Components|Activation|Activate _fx false :!label _label)
      (else
        (Components|Activation|Deactivate _fx :!label _label_2)))
    (elif (Variables|Default|GetIsDay?)
      (goto _label_2)
      (else
        (goto _label)))))

(event EventBeginPlay
  (|CallParentFunction)
  (bind _asmouse_character (Utilities|Casting|CastToMouseCharacter (Game|GetPlayerCharacter 0)))
  (Variables|Default|SetMainChar _asmouse_character)
  (EventDispatchers|BindEventtoDayNightSwitch _asmouse_character (delegate Custom|DayNightToggle))
  (bind _output_get (Variables|Default|SetDayOrNight (Actor|ActorHasTag "DayTP")))
  (if _output_get
    (bind _outactors (Actor|GetAllActorsOfClasswithTag "BP_MagicCircle_DayNight_C" "NightTP"))
    (Development|PrintString "GotNightTimeTags")
    (Variables|Default|SetTargetArray _outactors)
    (else
      (bind _outactors_2 (Actor|GetAllActorsOfClasswithTag "BP_MagicCircle_DayNight_C" "DayTP"))
      (Development|PrintString "GotDayTimeTags")
      (Variables|Default|SetTargetArray _outactors_2)
      (Components|Activation|Deactivate (Variables|Default|Getfx)))))

(event Collision|EventActorBeginOverlap
  (params (OtherActor :type Actor%20Object%20Reference))
  (|CallParentFunction OtherActor) ; This node is disabled and will not be called.\nDrag off pins to build functionality.
)

(event EventTick
  (params (DeltaSeconds :type Float%20%28single-precision%29))
  (|CallParentFunction DeltaSeconds))

(event EventTeleportToggle
  (Components|Activation|ToggleActive (Variables|Default|Getfx)))

(event EventTeleportColor
  ;[1 1 1] Change Circle Targeted Intensity (Scalar Param)
  (Effects|Components|ParticleSystem|SetFloatParameter (Variables|Default|Getfx) "color" (Math|Float|SelectFloat (Variables|Default|GetDefaultColor) 2e+02 (Variables|Default|GetIsColorSet?)))
  (if (Variables|Default|GetIsColorSet?)
    (Variables|Default|SetIsColorSet? false)
    (else
      (Variables|Default|SetIsColorSet? true))))

(fn ConstructionScript
  (|CallParentFunction)
  (Variables|Default|SetDefaultColor (Variables|Default|Getcolor)))