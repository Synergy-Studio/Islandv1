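; Player character Blueprint with walk, run, sprint and jump, plus cube pushing, switch interaction, teleporting and day/night cycling.
; Capsule overlaps and a facing check flag cube pushing, while a forward line trace messages switches.
; In two-way teleport mode, Tick picks targets by camera dot product and recolors them, then T hides, moves and reveals the player.
; Tab drives a sun-rotation timeline whose day/night state selects the target color array.
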(event OnComponentBeginOverlap(CapsuleComponent)
  (params (OverlappedComponent :type Primitive%20Component%20Object%20Reference) (OtherActor :type Actor%20Object%20Reference) (OtherComp :type Primitive%20Component%20Object%20Reference) (OtherBodyIndex :type Integer) (bFromSweep :type Boolean) (SweepResult :type Hit%20Result%20Structure%20%28by%20ref%29))
  ;[1 1 1] Push Cube Collision
  (Utilities|Casting|CastToPush_Cube_BP OtherActor)
  (Variables|Default|SetWhichCube (Components|GetOwner OtherComp))
  (Variables|Default|SetCanPushCube? true)
  (if (Variables|Default|GetRunning)
    (Variables|/Script/Engine.CharacterMovementComponent|SetMaxWalkSpeed (Variables|Character|GetCharacterMovement) 3e+02)))

(event OnComponentEndOverlap(CapsuleComponent)
  (params (OverlappedComponent :type Primitive%20Component%20Object%20Reference) (OtherActor :type Actor%20Object%20Reference) (OtherComp :type Primitive%20Component%20Object%20Reference) (OtherBodyIndex :type Integer))
  ;[1 1 1] Push Cube Collision
  (Utilities|Casting|CastToPush_Cube_BP OtherActor)
  (Variables|Default|SetCanPushCube? false)
  (Variables|Default|SetPushingCube false)
  (if (Variables|Default|GetRunning)
    (Variables|/Script/Engine.CharacterMovementComponent|SetMaxWalkSpeed (Variables|Character|GetCharacterMovement) 6e+02)))

(event EventTick
  (params (DeltaSeconds :type Float%20%28single-precision%29))
  ;[1 1 1] Event Tick
  (Development|PrintString (Utilities|String|ToString(Vector) (Transformation|GetActorLocation)) true true "(R=0.000000,G=0.660000,B=1.000000,A=1.000000)" DeltaSeconds)
  (if (Variables|Default|GetCanPushCube?)
    (if (>= (Math|Vector|DotProduct (Transformation|GetActorForwardVector) (Math|Vector|GetForwardVector (Math|Rotator|FindLookatRotation (Transformation|GetActorLocation) (Transformation|GetActorLocation (Variables|Default|GetWhichCube))))) 0.9)
      (Variables|Default|SetPushingCube true)
      (else
        (Variables|Default|SetPushingCube false))))
  (if (Variables|Default|GetCan2WayTele?)
    (bind _targetinview (CallFunction|2WayTargetting))
    (bind _output_get (Variables|Default|SetTargetInView _targetinview))
    (if _output_get
      (if (Variables|Default|GetTargetWidgetEnabled)
        _
        (else
          (Variables|Default|SetTargetWidgetEnabled true)))
      (elif (Variables|Default|GetTargetWidgetEnabled)
        (Variables|Default|SetTargetWidgetEnabled false))))
  (if (Variables|Default|GetJumping)
    (if (AI|Components|NavMovement|IsMovingonGround (Variables|Character|GetCharacterMovement))
      (Variables|Default|SetJumping false))))

(event EventBeginPlay
  ;[1 1 1] Event Begin Play
  (bind _outactors (Actor|GetAllActorsOfClass "/Game/Mechanics/FXVarietyPack/Blueprints/BP_ky_magicCircle1.BP_ky_magicCircle1_C"))
  (Variables|Default|SetTeleporters _outactors)
  (bind _outactors_2 (Actor|GetAllActorsOfClass "/Game/Mechanics/FXVarietyPack/Blueprints/BP_ky_magicCircle_Target.BP_ky_magicCircle_Target_C"))
  (bind _output_get (Variables|Default|SetTeleportTargets _outactors_2))
  (for (_ _array_index) _output_get
    (Utilities|Array|SetArrayElem (Variables|Default|GetIsColorSet?) _array_index false true))
  (bind _outactors_3 (Actor|GetAllActorsOfClasswithTag "/Game/Mechanics/FXVarietyPack/Blueprints/BP_MagicCircle_DayNight.BP_MagicCircle_DayNight_C" "DayTP"))
  (bind _output_get_2 (Variables|Default|SetNighttimeTargets _outactors_3))
  (for (_ _array_index_2) _output_get_2
    (Utilities|Array|SetArrayElem (Variables|Default|GetNighttimeColors) _array_index_2 false true))
  (bind _outactors_4 (Actor|GetAllActorsOfClasswithTag "/Game/Mechanics/FXVarietyPack/Blueprints/BP_MagicCircle_DayNight.BP_MagicCircle_DayNight_C" "NightTP"))
  (bind _output_get_3 (Variables|Default|SetDaytimeTargets _outactors_4))
  (for (_ _array_index_3) _output_get_3
    (Utilities|Array|SetArrayElem (Variables|Default|GetDaytimeColors) _array_index_3 false true)))

(event Event2WayTeleToggle
  (params (TargetsInReach :type Array%20of%20Actor%20Object%20References))
  ;[1 1 1] Teleport Toggles
  (Variables|Default|SetCan2WayTele? (not (Variables|Default|GetCan2WayTele?)))
  (Variables|Default|SetTargetsInView TargetsInReach))

(event EventTeleportToggle
  ;[1 1 1] Teleport Toggles
  (Variables|Default|SetCanTeleport? (not (Variables|Default|GetCanTeleport?))))

(event Input|ActionEvents|InputActionJump
  (params (Key :type Key%20Structure :default "None"))
  (bind _disabledmovement (Variables|Default|GetDisabledMovement))
  ;[1 1 1] Jump (Space)
  (:Pressed
    (if (not _disabledmovement)
      (if (not (Variables|Default|GetJumping))
        (Character|Jump)
        (Variables|Default|SetJumping true))))
  (:Released
    (if (not _disabledmovement)
      (Character|StopJumping))))

(event Input|ActionEvents|InputActionToggleRun
  (params (Key :type Key%20Structure :default "None"))
  (bind _charactermovement (Variables|Character|GetCharacterMovement))
  ;[1 1 1] Toggle Walk/Run (CapsLock)
  (:Pressed
    (bind _output_get (Variables|Default|SetRunning (not (Variables|Default|GetRunning))))
    (if _output_get
      (Variables|/Script/Engine.CharacterMovementComponent|SetMaxWalkSpeed _charactermovement 6e+02)
      (else
        (Variables|/Script/Engine.CharacterMovementComponent|SetMaxWalkSpeed _charactermovement 3e+02)))))

(event Input|ActionEvents|InputActionSprint
  (params (Key :type Key%20Structure :default "None"))
  (bind _charactermovement (Variables|Character|GetCharacterMovement))
  ;[1 1 1] Sprint (LeftShift)
  (:Pressed
    (Variables|Default|SetSprint true)
    (Variables|/Script/Engine.CharacterMovementComponent|SetMaxWalkSpeed _charactermovement 9e+02))
  (:Released
    (Variables|Default|SetSprint true)
    (if (Variables|Default|GetRunning)
      (Variables|/Script/Engine.CharacterMovementComponent|SetMaxWalkSpeed _charactermovement 6e+02)
      (else
        (Variables|/Script/Engine.CharacterMovementComponent|SetMaxWalkSpeed _charactermovement 2.5e+02)))))

(event Input|AxisEvents|InputAxisLookUp
  (params (AxisValue :type Float%20%28single-precision%29))
  ;[1 1 1] Mouse Camera Rotation
  (if (not (Variables|Default|GetDisabledMovement))
    (Pawn|Input|AddControllerPitchInput (* AxisValue (Utilities|Time|GetWorldDeltaSeconds) (Variables|Default|GetY_Sensitivity)))))

(event Input|AxisEvents|InputAxisLookUpRate
  (params (AxisValue :type Float%20%28single-precision%29))
  ;[1 1 1] Gamepad Camera Rotation
  (if (not (Variables|Default|GetDisabledMovement))
    (Pawn|Input|AddControllerPitchInput (* AxisValue (Utilities|Time|GetWorldDeltaSeconds) (Variables|Default|GetY_Sensitivity)))))

(event Input|AxisEvents|InputAxisTurn
  (params (AxisValue :type Float%20%28single-precision%29))
  ;[1 1 1] Mouse Camera Rotation
  (if (not (Variables|Default|GetDisabledMovement))
    (Pawn|Input|AddControllerYawInput (* AxisValue (Utilities|Time|GetWorldDeltaSeconds) (Variables|Default|GetX_Sensitivity)))))

(event Input|AxisEvents|InputAxisTurnRate
  (params (AxisValue :type Float%20%28single-precision%29))
  ;[1 1 1] Gamepad Camera Rotation
  (if (not (Variables|Default|GetDisabledMovement))
    (Pawn|Input|AddControllerYawInput (* AxisValue (Utilities|Time|GetWorldDeltaSeconds) (Variables|Default|GetX_Sensitivity)))))

(event Input|AxisEvents|InputAxisMoveForward
  (params (AxisValue :type Float%20%28single-precision%29))
  ;[1 1 1] Movement Control (WASD)
  (if (not (Variables|Default|GetDisabledMovement))
    (Pawn|Input|AddMovementInput (Math|Vector|GetForwardVector (Math|Rotator|MakeRotator 0.0 0.0 (.yaw (Pawn|GetControlRotation :!class /Script/Engine.Pawn)))) AxisValue false)))

(event Input|AxisEvents|InputAxisMoveRight
  (params (AxisValue :type Float%20%28single-precision%29))
  ;[1 1 1] Movement Control (WASD)
  (if (not (Variables|Default|GetDisabledMovement))
    (Pawn|Input|AddMovementInput (Math|Vector|GetRightVector (Math|Rotator|MakeRotator 0.0 0.0 (.yaw (Pawn|GetControlRotation :!class /Script/Engine.Pawn)))) (* AxisValue 0.5) false)))

(event Input|KeyboardEvents|P
  (params (Key :type Key%20Structure :default "None"))
  ;[1 1 1] Reload Level (P)
  (:Pressed
    (Game|OpenLevel(byName) "ThirdPersonExampleMap")))

(event Input|KeyboardEvents|E
  (params (Key :type Key%20Structure :default "None"))
  (bind _capsulecomponent (Variables|Collision|GetCapsuleComponent))
  (bind _returnvalue (Transformation|GetWorldLocation _capsulecomponent))
  ;[1 1 1] Switch Interaction (E)
  (:Pressed
    (if (not (Variables|Default|GetDisabledMovement))
      (bind (_outhit _returnvalue_2) (Collision|LineTraceByChannel _returnvalue (+ _returnvalue (* (Math|Vector|GetForwardVector (Transformation|GetWorldRotation _capsulecomponent)) 1.5e+02)) "TraceTypeQuery1" false 0 "ForDuration"))
      (if _returnvalue_2
        (Class|SwitchInterface|EnableSwitch(Message) (.HitActor (Collision|BreakHitResult _outhit)))))))

(event Input|KeyboardEvents|Tab
  (params (Key :type Key%20Structure :default "None"))
  ;[1 1 1] Cycle Day/Night (Tab)
  (:Pressed
    (if (not (Variables|Default|GetDisabledMovement))
      (if (Variables|Default|GetReadyToRotate)
        (Variables|Default|SetReadyToRotate false)
        (if (Variables|Default|GetDayNightToggle)
          (bind _rotatesun (Timeline|RotateSkySphere PlayFromStart)
            (:Update
              (Transformation|SetActorRotation (Variables|Default|GetLightSource) (Math|Rotator|MakeRotator 0.0 _rotatesun 0.0))
              (Default|UpdateSunDirection (Variables|Default|GetSkySphere)))
            (:Finished
              (if (Variables|Default|GetDayNightToggle)
                (Variables|Default|SetDayNightToggle false)
                (else
                  (Variables|Default|SetDayNightToggle true)))
              (Variables|Default|SetReadyToRotate true)
              (Default|CallDayNightSwitch)))
          (else
            (Timeline|RotateSkySphere ReverseFromEnd)))))))

(event Input|KeyboardEvents|O
  (params (Key :type Key%20Structure :default "None"))
  ;[1 1 1] Disable Movement (O)
  (:Pressed
    (if (Variables|Default|GetDisabledMovement)
      (Variables|Default|SetDisabledMovement false)
      (else
        (Variables|Default|SetDisabledMovement true)))))

(event Input|KeyboardEvents|T
  (params (Key :type Key%20Structure :default "None"))
  (bind _targettplocation (Variables|Default|GetTargetTPLocation))
  (bind _mesh (Variables|Character|GetMesh))
  (bind (_x _y _z) (Math|Vector|BreakVector _targettplocation))
  ;[1 1 1] Teleport Function (T)
  (:Pressed
    (if (and (or (Variables|Default|GetCanTeleport?) (Variables|Default|GetCan2WayTele?)) (Variables|Default|GetTargetInView))
      (Variables|Default|SetDisabledMovement true)
      (Rendering|SetVisibility _mesh false false)
      (Utilities|FlowControl|Delay 0.5)
      (Transformation|SetActorLocation (Math|Vector|MakeVector _x _y (+ _z (Variables|/Script/Engine.CapsuleComponent|GetCapsuleHalfHeight (Variables|Collision|GetCapsuleComponent)))) false true)
      (Rendering|SetVisibility _mesh true false)
      (Variables|Default|SetDisabledMovement false)
      (Variables|Default|SetCanTeleport? false)
      (Variables|Default|SetTargetWidgetEnabled false)
      (if (Variables|Default|GetCan2WayTele?)
        (Variables|Default|SetCan2WayTele? false)))))

(fn ConstructionScript)

(fn PushObject)

(fn BillboardTarget
  (bind _iscolorset_ (Variables|Default|GetIsColorSet?))
  (LocalVariables|SetTargetLocked false)
  (for (_array_element _array_index) (Variables|Default|GetTeleportTargets)
    (Development|PrintString (Utilities|String|Append (Utilities|GetDisplayName _array_element) ": " (Utilities|String|ToString(Float) (Math|Vector|DotProduct (Math|Vector|GetForwardVector (Transformation|GetActorRotation)) (Math|Vector|GetUnitDirection(Vector) (Transformation|GetActorLocation) (Transformation|GetActorLocation _array_element))))) true true "(R=0.000000,G=0.660000,B=1.000000,A=1.000000)" (Utilities|Time|GetWorldDeltaSeconds))
    (if (>= (Math|Vector|DotProduct (Math|Vector|GetForwardVector (Transformation|GetActorRotation)) (Math|Vector|GetUnitDirection(Vector) (Transformation|GetActorLocation) (Transformation|GetActorLocation _array_element))) 0.995)
      (Variables|Default|SetArrayIndex _array_index)
      (LocalVariables|SetTargetLocked true)
      (if (not (Utilities|Array|Get(acopy) (Variables|Default|GetIsColorSet?) _array_index))
        (Class|SwitchInterface|TeleportColor(Message) _array_element)
        (Variables|Default|SetTargetTPLocation (Transformation|GetActorLocation _array_element))
        (Utilities|Array|SetArrayElem _iscolorset_ _array_index true true))
      (elif (Utilities|Array|Get(acopy) (Variables|Default|GetIsColorSet?) _array_index)
        (Class|SwitchInterface|TeleportColor(Message) _array_element)
        (Utilities|Array|SetArrayElem _iscolorset_ _array_index false true))))
  (return (Variables|Default|GetArrayIndex) (LocalVariables|GetTargetLocked)))

(fn 2WayTargetting
  (bind _daynighttoggle (Variables|Default|GetDayNightToggle))
  (bind _maincam (Variables|Default|GetMainCam))
  (bind _daytimecolors (Variables|Default|GetDaytimeColors))
  (bind _nighttimecolors (Variables|Default|GetNighttimeColors))
  (bind _returnvalue (select _daynighttoggle _daytimecolors _nighttimecolors))
  (LocalVariables|SetTargetLocked false)
  (bind (_array_element _array_index) (Utilities|Array|ForEachLoopwithBreak (Variables|Default|GetTargetsInView) :!label _label)
    (:LoopBody
      (if (>= (Math|Vector|DotProduct (Math|Vector|GetForwardVector _maincam) (Math|Vector|GetUnitDirection(Vector) (Transformation|GetWorldLocation _maincam) (Transformation|GetActorLocation _array_element))) 0.99)
        (Variables|Default|SetArrayIndex _array_index)
        (LocalVariables|SetTargetLocked true)
        (if (Utilities|Array|Get(acopy) _returnvalue _array_index)
          (goto _label Break)
          (else
            (Class|SwitchInterface|TeleportColor(Message) _array_element)
            (bind _output_get (Variables|Default|SetTargetTPLocation (Transformation|GetActorLocation _array_element)))
            (Utilities|Array|SetArrayElem _returnvalue _array_index true true)
            (goto _label Break)))
        (elif (Utilities|Array|Get(acopy) _returnvalue _array_index)
          (Class|SwitchInterface|TeleportColor(Message) _array_element)
          (Utilities|Array|SetArrayElem _returnvalue _array_index false true))))
    (:Completed
      (return (Variables|Default|GetArrayIndex) (LocalVariables|GetTargetLocked) _output_get))))