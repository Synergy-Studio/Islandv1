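; Tree actor that slides horizontally away from the player (MouseCharacter) or the FollowTree AI and eases back toward its start position.
; Begin-overlap sets flags that gate Tick's distance checks and VInterpTo moves, with disperse steps clearing their flag.
; CreatePath shifts start positions within a fixed X band outward to split trees, but its BeamBP dispatcher binding is disconnected.
; Experimental left/right dot-product dodge logic is also disconnected.
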(event Custom|CreatePath
  (bind _returnvalue (Transformation|GetActorLocation))
  ;[1 1 1] Tree Seperation Event Dispatcher Event
  (bind (_shouldmove _updatedstartpoisition) (CallFunction|SeperateTrees))
  (if _shouldmove
    (Variables|Default|SetSeperateComplete false)
    (Variables|Default|SetStartingPosition _updatedstartpoisition)
    ;[1 1 1] Return Home
    (bind _returnvalue_2 (Transformation|SetActorLocation (Math|Vector|MakeVector (.x (Math|Interpolation|VInterpTo (Math|Vector|MakeVector (.x _returnvalue) (.y _returnvalue) (.z _returnvalue)) (Math|Vector|MakeVector (.X (Math|Vector|BreakVector (Variables|Default|GetStartingPosition))) (.Y (Math|Vector|BreakVector (Variables|Default|GetStartingPosition))) (.Z (Math|Vector|BreakVector (Variables|Default|GetStartingPosition)))) (Utilities|Time|GetWorldDeltaSeconds) 1.5)) (.y (Math|Interpolation|VInterpTo (Math|Vector|MakeVector (.x _returnvalue) (.y _returnvalue) (.z _returnvalue)) (Math|Vector|MakeVector (.X (Math|Vector|BreakVector (Variables|Default|GetStartingPosition))) (.Y (Math|Vector|BreakVector (Variables|Default|GetStartingPosition))) (.Z (Math|Vector|BreakVector (Variables|Default|GetStartingPosition)))) (Utilities|Time|GetWorldDeltaSeconds) 1.5)) (.z (Math|Interpolation|VInterpTo (Math|Vector|MakeVector (.x _returnvalue) (.y _returnvalue) (.z _returnvalue)) (Math|Vector|MakeVector (.X (Math|Vector|BreakVector (Variables|Default|GetStartingPosition))) (.Y (Math|Vector|BreakVector (Variables|Default|GetStartingPosition))) (.Z (Math|Vector|BreakVector (Variables|Default|GetStartingPosition)))) (Utilities|Time|GetWorldDeltaSeconds) 1.5))) false false))
    ;[1 1 1] Break tick event until move complete
    (Variables|Default|SetSeperateComplete true)))

(event Collision|EventActorBeginOverlap
  (params (OtherActor :type Actor%20Object%20Reference))
  ;[1 1 1] Check Player Overlapping
  (Variables|Default|SetOverlapping (Collision|IsOverlappingActor (Variables|Default|GetMainCharacter) :!class /Script/Engine.Actor))
  ;[1 1 1] Check AI Overlapping
  (Variables|Default|SetAIOverlap (Collision|IsOverlappingActor (Variables|Default|GetFollowTree) :!class /Script/Engine.Actor)))

(event EventTick
  (params (DeltaSeconds :type Float%20%28single-precision%29))
  (bind _returnvalue (Utilities|Time|GetWorldDeltaSeconds))
  (bind _returnvalue_2 (Transformation|GetActorLocation))
  (bind _returnvalue_3 (Utilities|Time|GetWorldDeltaSeconds))
  (bind _returnvalue_4 (Transformation|GetActorLocation))
  (bind _maincharacter (Variables|Default|GetMainCharacter))
  (bind _startingposition (Variables|Default|GetStartingPosition))
  (bind (_x _y _z) (Math|Vector|BreakVector _startingposition))
  (bind _returnvalue_5 (Transformation|GetActorLocation _maincharacter))
  (bind (_x_2 _y_2 _z_2) (Math|Vector|BreakVector _returnvalue_4))
  (bind _returnvalue_6 (Math|Interpolation|VInterpTo (Math|Vector|MakeVector (.x _returnvalue_2) (.y _returnvalue_2) (.z _returnvalue_2)) (Math|Vector|MakeVector _x _y _z) _returnvalue 1.5))
  (bind (_x_3 _y_3) (Math|Vector|BreakVector _returnvalue_5))
  (bind _returnvalue_7 (Math|Vector|GetUnitDirection(Vector) (Math|Vector|MakeVector _x_2 _y_2 0.0) (Math|Vector|MakeVector _x_3 _y_3 0.0)))
  (bind (_x_4 _y_4) (Math|Vector|BreakVector _returnvalue_7))
  (bind _returnvalue_8 (* (Math|Vector|MakeVector _x_4 _y_4 0.0) -4.5e+02))
  (bind _returnvalue_9 (+ (Math|Vector|MakeVector (.x _returnvalue_8) (.y _returnvalue_8) 0.0) (Math|Vector|MakeVector _x_3 _y_3 0.0)))
  (bind _returnvalue_10 (Math|Interpolation|VInterpTo (Math|Vector|MakeVector _x_2 _y_2 _z_2) (Math|Vector|MakeVector (.x _returnvalue_9) (.y _returnvalue_9) _z_2) _returnvalue_3 2.5))
  ;[1 1 1] AI Dispersion Function
  (if (Variables|Default|GetAIOverlap)
    (if (Variables|Default|GetSeperateComplete)
      (CallFunction|AIDisperse)))
  ;[1 1 1] Break Event if player not in range (Performance reasons)
  (if (Variables|Default|GetOverlapping)
    ;[1 1 1] Wait until separation is complete
    (if (Variables|Default|GetSeperateComplete)
      ;[1 1 1] Check tree is still in range of player (True: Disperse, False: Return Home)
      (if (< (Transformation|GetDistanceTo (Variables|Default|GetMainCharacter)) (Variables|Default|GetTreeColliderRadius))
        ;[1 1 1] Disperse
        (Transformation|SetActorLocation (Math|Vector|MakeVector (.x _returnvalue_10) (.y _returnvalue_10) (.z _returnvalue_10)) false false)
        (Variables|Default|SetOverlapping false)
        (else
          ;[1 1 1] Return Home
          (bind _returnvalue_11 (Transformation|SetActorLocation (Math|Vector|MakeVector (.x _returnvalue_6) (.y _returnvalue_6) (.z _returnvalue_6)) false false))
          ;[1 1 1] Break tick event until move complete
          (Variables|Default|SetSeperateComplete true))))))

(event EventBeginPlay
  (bind _returnvalue (Utilities|Time|GetWorldDeltaSeconds))
  (bind _returnvalue_2 (Transformation|GetActorLocation))
  (bind _startingposition (Variables|Default|GetStartingPosition))
  (bind (_x _y _z) (Math|Vector|BreakVector _startingposition))
  (bind _returnvalue_3 (Math|Interpolation|VInterpTo (Math|Vector|MakeVector (.x _returnvalue_2) (.y _returnvalue_2) (.z _returnvalue_2)) (Math|Vector|MakeVector _x _y _z) _returnvalue 1.5))
  (bind _asmouse_character (Utilities|Casting|CastToMouseCharacter (Game|GetPlayerCharacter 0)))
  ;[1 1 1] Set Tree Collider Radius & Player Character
  (Variables|Default|SetMainCharacter _asmouse_character)
  (Variables|Default|SetTreeColliderRadius (Components|Sphere|GetScaledSphereRadius (Variables|/Game/Blueprints/MouseCharacter/MouseCharacter.MouseCharacter_C|GetTreeCollider _asmouse_character)))
  ;[1 1 1] Set AICollider Radius
  (Variables|Default|SetAIColliderRadius (Components|Sphere|GetScaledSphereRadius (Variables|/Game/Blueprints/FollowTree_BP.FollowTree_BP_C|GetAICollider (Variables|Default|GetFollowTree))))
  ;[1 1 1] Return Home
  (bind _returnvalue_4 (Transformation|SetActorLocation (Math|Vector|MakeVector (.x _returnvalue_3) (.y _returnvalue_3) (.z _returnvalue_3)) false false))
  ;[1 1 1] Break tick event until move complete
  (Variables|Default|SetSeperateComplete true))

(fn ConstructionScript
  (Variables|Default|SetStartingPosition (Transformation|GetActorLocation)))

(fn SeperateTrees
  (Development|PrintString "EnteredFunction")
  (if (and (> (.x (Variables|Default|GetStartingPosition)) -1.7e+03) (< (.x (Variables|Default|GetStartingPosition)) -1.2e+03))
    (if (> (.x (Variables|Default|GetStartingPosition)) -1.45e+03)
      (bind _output_get (Variables|Default|SetStartingPosition (Math|Vector|MakeVector (+ (.x (Variables|Default|GetStartingPosition)) 4e+02) (.y (Variables|Default|GetStartingPosition)) (.z (Variables|Default|GetStartingPosition)))))
      (Development|PrintString "SplitTrees")
      (return true _output_get)
      (else
        (bind _output_get_2 (Variables|Default|SetStartingPosition (Math|Vector|MakeVector (- (.x (Variables|Default|GetStartingPosition)) 4e+02) (.y (Variables|Default|GetStartingPosition)) (.z (Variables|Default|GetStartingPosition)))))
        (Development|PrintString "SplitTrees")
        (return true _output_get_2)))
    (else
      (return false (Math|Vector|MakeVector (.x (Variables|Default|GetStartingPosition)) (.y (Variables|Default|GetStartingPosition)) (.z (Variables|Default|GetStartingPosition)))))))

(fn AIDisperse
  (bind _returnvalue (Utilities|Time|GetWorldDeltaSeconds))
  (bind _returnvalue_2 (Transformation|GetActorLocation))
  (bind _returnvalue_3 (Utilities|Time|GetWorldDeltaSeconds))
  (bind _returnvalue_4 (Transformation|GetActorLocation))
  (bind _followtree (Variables|Default|GetFollowTree))
  (bind _followtree_2 (Variables|Default|GetFollowTree))
  (bind _startingposition (Variables|Default|GetStartingPosition))
  (bind (_x _y) (Math|Vector|BreakVector _startingposition))
  (bind _returnvalue_5 (Transformation|GetActorLocation _followtree))
  (bind _returnvalue_6 (Transformation|GetActorLocation _followtree_2))
  (bind (_x_2 _y_2 _z) (Math|Vector|BreakVector _returnvalue_4))
  (bind _returnvalue_7 (Math|Interpolation|VInterpTo (Math|Vector|MakeVector (.x _returnvalue_2) (.y _returnvalue_2) (.z _returnvalue_2)) (Math|Vector|MakeVector _x _y (.z _returnvalue_2)) _returnvalue 1.5))
  (bind (_x_3 _y_3) (Math|Vector|BreakVector _returnvalue_6))
  (bind _returnvalue_8 (Math|Vector|GetUnitDirection(Vector) (Math|Vector|MakeVector _x_2 _y_2 0.0) (Math|Vector|MakeVector _x_3 _y_3 0.0)))
  (bind (_x_4 _y_4) (Math|Vector|BreakVector _returnvalue_8))
  (bind _returnvalue_9 (* (Math|Vector|MakeVector _x_4 _y_4 0.0) -4.5e+02))
  (bind _returnvalue_10 (+ (Math|Vector|MakeVector (.x _returnvalue_9) (.y _returnvalue_9) 0.0) (Math|Vector|MakeVector _x_3 _y_3 0.0)))
  (bind _returnvalue_11 (Math|Interpolation|VInterpTo (Math|Vector|MakeVector _x_2 _y_2 _z) (Math|Vector|MakeVector (.x _returnvalue_10) (.y _returnvalue_10) _z) _returnvalue_3 2.5))
  ;[1 1 1] Get Distance To AI Actor
  (if (< (Transformation|GetDistanceTo _followtree) (Variables|Default|GetAIColliderRadius))
    ;[1 1 1] Disperse
    (Transformation|SetActorLocation (Math|Vector|MakeVector (.x _returnvalue_11) (.y _returnvalue_11) (.z _returnvalue_11)) false false)
    (Variables|Default|SetAIOverlap false)
    (return)
    (else
      ;[1 1 1] Get AI position and break return home if x,y not changed since last tick
      (if (not (Math|Vector|Equal(Vector) _returnvalue_5 (Variables|Default|GetAILastPosition) 1.0))
        (Variables|Default|SetAILastPosition _returnvalue_5)
        ;[1 1 1] Return Home
        (Transformation|SetActorLocation (Math|Vector|MakeVector (.x _returnvalue_7) (.y _returnvalue_7) (.z _returnvalue_7)) false false)
        (return)))))