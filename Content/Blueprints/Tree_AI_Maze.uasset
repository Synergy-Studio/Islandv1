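; AI tree for a maze that retreats when the player's MouseCharacter touches its capsule, then returns to its starting spot.
; Impulse uses the navmesh to move it 500 units along the direction away from the player, printing debug results.
; While away from home, Tick repeats Impulse during overlap, otherwise sends it back once the player is outside a 450-unit tolerance of the start.
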(event OnComponentBeginOverlap(CapsuleComponent)
  (params (OverlappedComponent :type Primitive%20Component%20Object%20Reference) (OtherActor :type Actor%20Object%20Reference) (OtherComp :type Primitive%20Component%20Object%20Reference) (OtherBodyIndex :type Integer) (bFromSweep :type Boolean) (SweepResult :type Hit%20Result%20Structure%20%28by%20ref%29))
  (Utilities|Casting|CastToMouseCharacter OtherActor)
  (Variables|Default|SetMainCharCollider OtherComp)
  (CallFunction|Impulse)
  (Variables|Default|SetAtHome? false))

(event EventBeginPlay
  (bind _asmouse_character (Utilities|Casting|CastToMouseCharacter (Game|GetPlayerCharacter 0)))
  (Variables|Default|SetMainChar _asmouse_character)
  (Variables|Default|SetStartingPosition (Transformation|GetActorLocation)))

(event EventTick
  (params (DeltaSeconds :type Float%20%28single-precision%29))
  (if (not (Variables|Default|GetAtHome?))
    (if (Class|PrimitiveComponent|IsOverlappingComponent (Variables|Collision|GetCapsuleComponent) (Variables|Default|GetMainCharCollider))
      (CallFunction|Impulse)
      (Variables|Default|SetAtHome? false)
      (elif (not (Math|Vector|Equal(Vector) (Variables|Default|GetStartingPosition) (Transformation|GetActorLocation (Variables|Default|GetMainChar)) 4.5e+02))
        (AI|AIMoveTo self (Variables|Default|GetStartingPosition) 0 1.0 true
          (:OnSuccess
            (Variables|Default|SetAtHome? true))
          (:OnFail
            (Variables|Default|SetAtHome? false)))))))

(fn ConstructionScript)

(fn Impulse
  (bind _returnvalue (Utilities|Time|GetWorldDeltaSeconds))
  (bind _returnvalue_2 (Transformation|GetActorLocation))
  (bind _mainchar (Variables|Default|GetMainChar))
  (bind _returnvalue_3 (Transformation|GetActorLocation _mainchar))
  (bind _z (Math|Vector|BreakVector _returnvalue_2))
  (bind _returnvalue_4 (Math|Rotator|FindLookatRotation _returnvalue_3 _returnvalue_2))
  (bind _returnvalue_5 (Math|Vector|GetForwardVector _returnvalue_4))
  (bind _returnvalue_6 (* _returnvalue_5 5e+02))
  (bind _returnvalue_7 (Math|Vector|MakeVector (.x _returnvalue_6) (.y _returnvalue_6) _z))
  (bind _returnvalue_8 (+ _returnvalue_7 _returnvalue_2))
  (bind _returnvalue_9 (AI|Navigation|MovetoLocation (AI|GetAIController self) _returnvalue_8 1.0 true true false true "/Script/AIModule.NavFilter_AIControllerDefault"))
  (Development|PrintString (Utilities|String|Append "DidMove: " (Utilities|String|EnumtoString _returnvalue_9)) true true "(R=0.000000,G=0.660000,B=1.000000,A=1.000000)" _returnvalue)
  (Development|PrintString (Utilities|String|Append "Destination: " (Utilities|String|ToString(Vector) _returnvalue_8)) true true "(R=0.000000,G=0.660000,B=1.000000,A=1.000000)" _returnvalue)
  (return))