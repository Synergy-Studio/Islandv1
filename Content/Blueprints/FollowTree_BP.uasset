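; Tree actor that starts creeping after the MouseCharacter on overlap, advancing only while the player faces away from it.
; Tick yaws it toward the player, using a forward-vector dot product to gate movement, then interpolates XY once roughly aligned and beyond close range.
; Exceeding MaxDistance from the start clears ShouldFollow, so it turns, glides back to the transform saved in the Construction Script and restores its yaw.
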(event Collision|EventActorBeginOverlap
  (params (OtherActor :type Actor%20Object%20Reference))
  (Utilities|Casting|CastToMouseCharacter OtherActor)
  ;[1 1 1] Trigger follow when collision occurs
  (if (> (Math|Vector|Distance(Vector) (Variables|Default|GetStartingPosition) (Transformation|GetActorLocation)) (Variables|Default|GetMaxDistance))
    (Variables|Default|SetShouldFollow false)
    (else
      (Variables|Default|SetShouldFollow true))))

(event EventTick
  (params (DeltaSeconds :type Float%20%28single-precision%29))
  (bind _returnvalue (Transformation|GetActorLocation))
  (bind _returnvalue_2 (Transformation|GetActorRotation))
  (bind _returnvalue_3 (Transformation|GetActorLocation))
  (bind _returnvalue_4 (Utilities|Time|GetWorldDeltaSeconds))
  (bind _returnvalue_5 (Transformation|GetActorRotation))
  (bind _returnvalue_6 (Transformation|GetActorRotation))
  (bind _returnvalue_7 (Transformation|GetActorLocation))
  (bind _returnvalue_8 (Utilities|Time|GetWorldDeltaSeconds))
  (bind _returnvalue_9 (Transformation|GetActorRotation))
  (bind _startingposition (Variables|Default|GetStartingPosition))
  (bind _startingposition_2 (Variables|Default|GetStartingPosition))
  (bind _playercharacter (Variables|Default|GetPlayerCharacter))
  (bind _playercharacter_2 (Variables|Default|GetPlayerCharacter))
  (bind (_x _y _z) (Math|Vector|BreakVector _startingposition_2))
  (bind _returnvalue_10 (Transformation|GetActorLocation _playercharacter_2))
  (bind (_x_2 _y_2) (Math|Vector|BreakVector _returnvalue))
  (bind _returnvalue_11 (Math|Rotator|FindLookatRotation _returnvalue_7 _startingposition))
  (bind _returnvalue_12 (Math|Interpolation|VInterpTo (Math|Vector|MakeVector (.x _returnvalue_3) (.y _returnvalue_3) 0.0) (Math|Vector|MakeVector (.x _returnvalue_10) (.y _returnvalue_10) 0.0) _returnvalue_4 1.5))
  (bind _returnvalue_13 (Math|Interpolation|VInterpTo (Math|Vector|MakeVector _x_2 _y_2 _z) (Math|Vector|MakeVector _x _y _z) _returnvalue_8 0.5))
  (if (Variables|Default|GetShouldFollow)
    ;[1 1 1] LookAt Player (Rotate)
    (Transformation|SetActorRotation (Math|Interpolation|RInterpTo (Math|Rotator|MakeRotator (.roll _returnvalue_2) (.pitch _returnvalue_2) (.yaw _returnvalue_2)) (Math|Rotator|MakeRotator (.roll _returnvalue_2) (.pitch _returnvalue_2) (.yaw (Math|Rotator|FindLookatRotation (Transformation|GetActorLocation) (Transformation|GetActorLocation (Variables|Default|GetPlayerCharacter))))) (Utilities|Time|GetWorldDeltaSeconds) 2.5))
    ;[1 1 1] Check Players LookAt Vector
    (if (>= (Math|Vector|DotProduct (Transformation|GetActorForwardVector) (Transformation|GetActorForwardVector _playercharacter)) 0.0)
      ;[1 1 1] Check Distance to Player
      (if (not (<= (Transformation|GetDistanceTo _playercharacter) 3e+02))
        ;[1 1 1] Check tree hasn't reached max distance from starting position
        (if (> (Math|Vector|Distance(Vector) (Variables|Default|GetStartingPosition) (Transformation|GetActorLocation)) (Variables|Default|GetMaxDistance))
          (Variables|Default|SetShouldFollow false)
          (else
            ;[1 1 1] Rotate before beginning to move
            (if (Math|Rotator|Equal(Rotator) (Math|Rotator|MakeRotator (.roll _returnvalue_5) (.pitch _returnvalue_5) (.yaw _returnvalue_5)) (Math|Rotator|MakeRotator (.roll _returnvalue_5) (.pitch _returnvalue_5) (.yaw (Math|Rotator|FindLookatRotation (Transformation|GetActorLocation) (Math|Vector|MakeVector (.x _returnvalue_10) (.y _returnvalue_10) (.z _returnvalue_10))))) 2e+01)
              ;[1 1 1] Interp to player position
              (Transformation|SetActorLocation (Math|Vector|MakeVector (.x _returnvalue_12) (.y _returnvalue_12) (.z _returnvalue_3)) false false))))))
    (elif (Math|Vector|Equal(Vector) _startingposition _returnvalue_7 1e+01)
      ;[1 1 1] Reset to Starting Position LookAt (Rotate)
      (Transformation|SetActorRotation (Math|Interpolation|RInterpTo (Math|Rotator|MakeRotator (.roll _returnvalue_9) (.pitch _returnvalue_9) (.yaw _returnvalue_9)) (Math|Rotator|MakeRotator (.roll _returnvalue_9) (.pitch _returnvalue_9) (.Yaw (Math|Rotator|BreakRotator (Variables|Default|GetStartingRotation)))) (Utilities|Time|GetWorldDeltaSeconds) 3.5))
      (else
        ;[1 1 1] LookAt Starting Position (Rotate)
        (Transformation|SetActorRotation (Math|Interpolation|RInterpTo (Math|Rotator|MakeRotator (.roll _returnvalue_6) (.pitch _returnvalue_6) (.yaw _returnvalue_6)) (Math|Rotator|MakeRotator (.roll _returnvalue_6) (.pitch _returnvalue_6) (.yaw _returnvalue_11)) (Utilities|Time|GetWorldDeltaSeconds) 2.5))
        ;[1 1 1] Rotate before beginning to move
        (if (Math|Rotator|Equal(Rotator) (Math|Rotator|MakeRotator (.roll _returnvalue_6) (.pitch _returnvalue_6) (.yaw _returnvalue_6)) (Math|Rotator|MakeRotator (.roll _returnvalue_6) (.pitch _returnvalue_6) (.yaw _returnvalue_11)) 1e+01)
          ;[1 1 1] Return to starting position
          (Transformation|SetActorLocation (Math|Vector|MakeVector (.x _returnvalue_13) (.y _returnvalue_13) (.z _returnvalue_13)) false false))))))

(event EventBeginPlay
  (bind _asmouse_character (Utilities|Casting|CastToMouseCharacter (Game|GetPlayerCharacter 0)))
  (Variables|Default|SetPlayerCharacter _asmouse_character))

(fn ConstructionScript
  (Variables|Default|SetStartingPosition (Transformation|GetActorLocation))
  (Variables|Default|SetStartingRotation (Transformation|GetActorRotation)))